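; NPC AI controller that runs BT_NPC and feeds perception results into its blackboard to track the player.
; Sight and hearing set or clear TargetActor as the player, though hearing never checks which actor made the sound.
; Losing sight requests a one-second prediction, whose stimulus location is saved as LastKnowLocation.
; The touch handler is never run, and a debug sphere draws at TargetLocation, a key this controller never writes.
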(event OnTargetPerceptionUpdated(AIPerception)
  (params (Actor :type Actor%20Object%20Reference) (Stimulus :type AI%20Stimulus%20Structure))
  (CallFunction|HandleSightSense Actor Stimulus)
  (CallFunction|HandleSoundDetection Stimulus)
  (CallFunction|HandlePrediction Stimulus)
  (Rendering|Debug|DrawDebugSphere (AI|Components|Blackboard|GetValueasVector (AI|GetBlackboard 0) (Utilities|Name|MakeLiteralName "TargetLocation")) 1e+02 12 "(R=1.000000,G=0.081730,B=0.201468,A=1.000000)" 2.0))

(event EventBeginPlay
  (AI|RunBehaviorTree "/Game/Characters/Ai/BehaviorTree/BT_NPC.BT_NPC"))

(fn ConstructionScript)

(fn HandleSightSense
  (params (Actor :type Actor%20Object%20Reference) (Stimulus :type AI%20Stimulus%20Structure))
  (bind _returnvalue (Class|AIPerceptionSystem|GetSenseClassforStimulus Stimulus))
  (if (== _returnvalue "/Script/AIModule.AISense_Sight")
    (if (== Actor (Game|GetPlayerCharacter 0))
      (AI|Components|Blackboard|SetValueasObject (Variables|Default|GetBlackboard) (Utilities|Name|MakeLiteralName "TargetActor") (Utilities|SelectObject (Game|GetPlayerCharacter 0) 0 (.bsuccessfullysensed Stimulus)))
      (if (not (.bsuccessfullysensed Stimulus))
        (Class|AISensePrediction|RequestPawnPredictionEvent (Pawn|GetControlledPawn) (Game|GetPlayerCharacter 0) 1.0))
      (else
        (return) ; If it is not the actor we return
      ))
    (else
      (return) ; If the senses doesn't match, return
    )))

(fn HandleSoundDetection
  (params (Stimulus :type AI%20Stimulus%20Structure%20%28by%20ref%29))
  (bind _returnvalue (Class|AIPerceptionSystem|GetSenseClassforStimulus Stimulus))
  (if (== _returnvalue "/Script/AIModule.AISense_Hearing")
    (AI|Components|Blackboard|SetValueasObject (Variables|Default|GetBlackboard) (Utilities|Name|MakeLiteralName "TargetActor") (Utilities|SelectObject (Game|GetPlayerCharacter 0) 0 (.bsuccessfullysensed Stimulus)))))

(fn HandlePrediction
  (params (Stimulus :type AI%20Stimulus%20Structure%20%28by%20ref%29))
  (bind _returnvalue (Class|AIPerceptionSystem|GetSenseClassforStimulus Stimulus))
  (if (== _returnvalue "/Script/AIModule.AISense_Prediction")
    (AI|Components|Blackboard|SetValueasVector (Variables|Default|GetBlackboard) (Utilities|Name|MakeLiteralName "LastKnowLocation") (.StimulusLocation (Utilities|Struct|BreakAIStimulus Stimulus)))))

(fn HandleTouchEvent
  (params (Actor :type Actor%20Object%20Reference) (Stimulus :type AI%20Stimulus%20Structure))
  (bind _returnvalue (Class|AIPerceptionSystem|GetSenseClassforStimulus Stimulus))
  (if (== _returnvalue "/Script/AIModule.AISense_Touch")
    (if (== Actor (Game|GetPlayerCharacter 0))
      (AI|Components|Blackboard|SetValueasObject (Variables|Default|GetBlackboard) (Utilities|Name|MakeLiteralName "TargetActor") (Utilities|SelectObject (Game|GetPlayerCharacter 0) 0 (.bsuccessfullysensed Stimulus)))
      (else
        (return) ; If it is not the actor we return
      ))
    (else
      (return) ; If it is not the actor we return
    )))