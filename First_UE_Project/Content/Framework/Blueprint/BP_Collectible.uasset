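; BP_Collectible is a coin pickup that bounces and spins in place.
; A timeline started on BeginPlay drives the Centerpoint component's height and yaw each update.
; When the player character overlaps its Box, it calls OnCoinPickUp on BP_GameMode and destroys itself.
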(event OnComponentBeginOverlap(Box)
  (params (OverlappedComponent :type Primitive%20Component%20Object%20Reference) (OtherActor :type Actor%20Object%20Reference) (OtherComp :type Primitive%20Component%20Object%20Reference) (OtherBodyIndex :type Integer) (bFromSweep :type Boolean) (SweepResult :type Hit%20Result%20Structure%20%28by%20ref%29))
  (if (== OtherActor (Game|GetPlayerCharacter 0))
    (bind _asbp_game_mode (Utilities|Casting|CastToBP_GameMode (Game|GetGameMode)))
    (Default|OnCoinPickUp _asbp_game_mode)
    (Actor|DestroyActor)))

(event EventBeginPlay
  (bind (_direction _bounceheight _gyro) (Timeline|RotationAnimation PlayFromStart)
    (:Update
      (Transformation|SetRelativeTransform (Variables|Default|GetCenterpoint) (Math|Transform|MakeTransform (Math|Vector|MakeVector 0.0 0.0 _bounceheight) (Math|Rotator|MakeRotator 0.0 0.0 (.z _gyro)) "1.000000,1.000000,1.000000") false false))))

(fn ConstructionScript)