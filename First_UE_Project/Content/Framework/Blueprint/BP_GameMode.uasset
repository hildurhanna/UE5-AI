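; Game mode for a timed coin-collecting game with levels, driving intro, HUD and game-over widgets.
; After a Get Ready/Go intro, Tick counts down the timer and quits the game at zero.
; Coin pickups add level-scaled points, retry a random TargetPoint occupancy check until a replacement spawns, then may level up for bonus time.
; Win checking is an empty stub; coin reshuffling is unwired.
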(event Custom|AddPoint
  ;[1 1 1] Adding points
  (Variables|Default|SetPoint (+ (* (Variables|Default|GetPlayerLevel) 10) (Variables|Default|GetPoint))))

(event Custom|LevelUp
  (if (and (== (Math|Integer|%(Integer) (Variables|Default|GetTotalAmountOfCoins) (Variables|Default|GetCoinsToLevelComplete)) 0) (< (Variables|Default|GetPlayerLevel) 5))
    (bind _result (Math|Integer|IncrementInt (Variables|Default|GetPlayerLevel))
      (:%20%20
        (CallFunction|UpdateLevelPoints _result)
        (Variables|Default|SetTimeLeft (+ (Variables|Default|GetTimeLeft) 15.0))))))

(event Custom|Countdown_OnTick
  ;[1 1 1] Countdown per tick
  (Variables|Default|SetTimeLeft (- (Variables|Default|GetTimeLeft) (Utilities|Time|GetWorldDeltaSeconds))))

(event Custom|InitializeSequence
  ;[1 1 1] Prepare the player for startup
  (CallFunction|OnGetReady)
  (Utilities|FlowControl|Delay 2.0)
  (CallFunction|OnStart)
  (Variables|Default|SetIsGameActive true)
  (Actor|Tick|SetActorTickEnabled true)
  (CallFunction|ShowUI))

(event Custom|InitializeGameRules
  (bind _outactors (Actor|GetAllActorsOfClass "/Game/Characters/BP_Collectible.BP_Collectible_C"))
  (Variables|Default|SetTotalAmountOfCoins (Utilities|Array|Length _outactors)))

(event Custom|OnCoinPickUp
  ;[1 1 1] When the player picks upp coin
  (CallFunction|AddPoint)
  (Math|Integer|IncrementInt (Variables|Default|GetTotalAmountOfCoins)
    (:%20%20
      (CallFunction|UpdateUIPoints (Variables|Default|GetPoint))
      (bind _success (CallFunction|CheckTargetAvailabilityandSpawnCoin :!label _label))
      (if _success
        (CallFunction|LevelUp)
        (else
          (goto _label))))))

(event Custom|CheckWinningCondition
  ;[1 1 1] Check if the player has won or lost
)

(event Custom|CheckTimeLeft
  ;[1 1 1] Check the time status
  (if (<= (Variables|Default|GetTimeLeft) 0.0)
    (Variables|Default|SetIsGameActive false)
    (CallFunction|CheckWinningCondition)
    ;[1 1 1] Gives game over when the time is up
    (CallFunction|OnGameOver)
    (Actor|Tick|SetActorTickEnabled false)
    (CallFunction|ShowUI)
    (Utilities|FlowControl|Delay 1.0)
    (Game|QuitGame 0 "Quit" false)))

(event Custom|LevelDelay
  (Utilities|FlowControl|Delay (Math|Conversions|ToFloat(Integer) (- 6 (Variables|Default|GetPlayerLevel))))
  (bind _outactors (Actor|GetAllActorsOfClass "/Game/Characters/BP_Collectible.BP_Collectible_C"))
  (for _array_element _outactors
    (bind _outactors_2 (Actor|GetAllActorsOfClass "/Script/Engine.TargetPoint"))
    (Transformation|SetActorTransform _array_element (Transformation|GetActorTransform (Utilities|Array|Get(acopy) _outactors_2 (Math|Random|RandomIntegerinRange 0 (Utilities|Array|LastIndex _outactors_2)))) false true)))

(event EventTick
  (params (DeltaSeconds :type Float%20%28single-precision%29))
  ;[1 1 1] Countdown per tick
  (CallFunction|CountdownonTick)
  (CallFunction|CheckTimeLeft)
  (CallFunction|UIUpdate))

(event EventBeginPlay
  (CallFunction|InitializeGameRules)
  (CallFunction|InitializeSequence)
  (CallFunction|InitializeUI)
  ;[1 1 1] When the player picks upp coin
  (CallFunction|UpdateLevelPoints (Variables|Default|GetPlayerLevel)))

(event Custom|InitializeUI
  (bind _returnvalue (UserInterface|CreateWidget "/Game/UI/UI_Game.UI_Game_C" (Game|GetPlayerController 0)))
  (Variables|Default|SetUIRef _returnvalue))

(event Custom|ShowUI
  (UserInterface|Viewport|AddtoViewport (Variables|Default|GetUIRef) 0))

(event Custom|UpdateUITime
  (params (Time :type Float%20%28double-precision%29))
  (Rendering|Components|TextRender|SetText (Variables|/Game/UI/UI_Game.UI_Game_C|GetTimeValue (Variables|Default|GetUIRef)) (Utilities|Text|ToText(Float) Time "HalfToEven")))

(event Custom|UpdateUIPoints
  (params (Points :type Integer))
  (Rendering|Components|TextRender|SetText (Variables|/Game/UI/UI_Game.UI_Game_C|GetPointsValue (Variables|Default|GetUIRef)) (Utilities|Text|ToText(Integer) Points)))

(event Custom|UIUpdate
  ;[1 1 1] On Coundown Tick
  (CallFunction|UpdateUITime (Variables|Default|GetTimeLeft)))

(event Custom|OnGetReady
  ;[1 1 1] Get Ready Go Animation
  (bind _returnvalue (UserInterface|CreateWidget "/Game/UI/UI_GetReadyGo.UI_GetReadyGo_C" (Game|GetPlayerController 0)))
  (bind _output_get (Variables|Default|SetGetReadyGoRef _returnvalue))
  (UserInterface|Viewport|AddtoViewport _output_get 0)
  (Default|PlayGetReadyText _output_get))

(event Custom|OnStart
  ;[1 1 1] Get Ready Go Animation
  (Default|PlayGoText (Variables|Default|GetGetReadyGoRef)))

(event Custom|OnGameOver
  ;[1 1 1] Game Over Animation
  (bind _returnvalue (UserInterface|CreateWidget "/Game/UI/GameOver.GameOver_C" (Game|GetPlayerController 0)))
  (bind _output_get (Variables|Default|SetGetGameOverRef _returnvalue))
  (UserInterface|Viewport|AddtoViewport _output_get 0)
  (Default|PlayGameOver _output_get))

(event Custom|UpdateLevelPoints
  (params (Level :type Integer))
  (Rendering|Components|TextRender|SetText (Variables|/Game/UI/UI_Game.UI_Game_C|GetLevelValue (Variables|Default|GetUIRef)) (Utilities|Text|ToText(Integer) Level)))

(fn ConstructionScript)

(fn CheckTargetAvailabilityandSpawnCoin
  (bind _outactors (Actor|GetAllActorsOfClass "/Script/Engine.TargetPoint")) ; Here we get all the target points
  (bind _outactors_2 (Actor|GetAllActorsOfClass "/Game/Characters/BP_Collectible.BP_Collectible_C"))
  (bind _array_element (Utilities|Array|ForEachLoopwithBreak _outactors_2 :!label _label)
    (:LoopBody
      ;[1 1 1] is chosen target point already occupied?
      (if (Utilities|Operators|EqualEqual (Transformation|GetActorLocation _array_element) (Transformation|GetActorLocation (Utilities|Array|Get(acopy) _outactors (Math|Random|RandomIntegerinRange 0 (Utilities|Array|LastIndex _outactors)))) 5.0)
        (Utilities|FlowControl|Sequence
          (:then_0
            (LocalVariables|SetFoundOverlappingTargetPoint true)
            (if (LocalVariables|GetFoundOverlappingTargetPoint) :!label _label_2
              (return false)
              (else
                (Game|SpawnActorfromClass "/Game/Characters/BP_Collectible.BP_Collectible_C" (Math|Transform|MakeTransform (.location (Transformation|GetActorTransform (Utilities|Array|Get(acopy) _outactors (Math|Random|RandomIntegerinRange 0 (Utilities|Array|LastIndex _outactors))))) "0, 0, 0" "1.000000,1.000000,1.000000") "Undefined" "MultiplyWithRoot" 0 0)
                (return true))))
          (:then_1
            (goto _label Break)))))
    (:Completed
      (goto _label_2))))

(fn GetRandomTargetLocation
  (bind _outactors (Actor|GetAllActorsOfClass "/Script/Engine.TargetPoint" :!label _label))
  (LocalVariables|SetTempTargetPoint (Utilities|Array|Get(acopy) _outactors (Math|Random|RandomIntegerinRange 0 (Utilities|Array|LastIndex _outactors))))
  (bind _outactors_2 (Actor|GetAllActorsOfClass "/Game/Characters/BP_Collectible.BP_Collectible_C"))
  (bind _array_element (Utilities|Array|ForEachLoopwithBreak _outactors_2 :!label _label_2)
    (:LoopBody
      ;[1 1 1] is chosen target point already occupied?
      (if (Utilities|Operators|EqualEqual (Transformation|GetActorLocation _array_element) (Transformation|GetActorLocation (LocalVariables|GetTempTargetPoint)) 0.0)
        (Utilities|FlowControl|Sequence
          (:then_0
            (Development|PrintString "Hello")
            (goto _label_2 Break))
          (:then_1
            (goto _label)))))
    (:Completed
      (return (LocalVariables|GetTempTargetPoint)))))