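; Player character Blueprint that handles movement, look and jump through Enhanced Input and can respawn itself as a new character.
; BeginPlay adds the PlayerMainGame mapping context to player 0, and input actions drive jumping, movement along the actor's forward and right vectors, and controller yaw and pitch.
; Pressing F asks BP_PlayerController to spawn a new character, then destroys this one.
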(event Input|EnhancedActionEvents|EnhancedInputActionPlayerMovement
  (params (ActionValue :type Vector%202D%20Structure) (ElapsedSeconds :type Float%20%28double-precision%29) (TriggeredSeconds :type Float%20%28double-precision%29) (InputAction :type Input%20Action%20Object%20Reference :default "/Game/Framework/Input/PlayerMovement.PlayerMovement"))
  (:Triggered
    (Utilities|FlowControl|Sequence
      (:then_0
        (Pawn|Input|AddMovementInput (Transformation|GetActorForwardVector) (.x ActionValue) false))
      (:then_1
        (Pawn|Input|AddMovementInput (Transformation|GetActorRightVector) (.y ActionValue) false)))))

(event Input|EnhancedActionEvents|EnhancedInputActionPlayerJump
  (params (ActionValue :type Boolean) (ElapsedSeconds :type Float%20%28double-precision%29) (TriggeredSeconds :type Float%20%28double-precision%29) (InputAction :type Input%20Action%20Object%20Reference :default "/Game/Framework/Input/PlayerJump.PlayerJump"))
  (:Triggered
    (Character|Jump)))

(event Input|EnhancedActionEvents|EnhancedInputActionIA_PlayerLook
  (params (ActionValue :type Vector%202D%20Structure) (ElapsedSeconds :type Float%20%28double-precision%29) (TriggeredSeconds :type Float%20%28double-precision%29) (InputAction :type Input%20Action%20Object%20Reference :default "/Game/Framework/Input/IA_PlayerLook.IA_PlayerLook"))
  (:Triggered
    (Pawn|Input|AddControllerYawInput (.x ActionValue))
    (Pawn|Input|AddControllerPitchInput (.y ActionValue))))

(event EventBeginPlay
  (Input|AddMappingContext (PlayerController|LocalPlayerSubsystems|GetEnhancedInputLocalPlayerSubsystem (Game|GetPlayerController 0)) "/Game/Framework/Input/PlayerMainGame.PlayerMainGame" 0 "(bIgnoreAllPressedKeysUntilRelease=True,bForceImmediately=False)"))

(event Input|KeyboardEvents|F
  (params (Key :type Key%20Structure :default "None"))
  (:Pressed
    (bind _asbp_player_controller (Utilities|Casting|CastToBP_PlayerController (Pawn|GetController)))
    (Default|SpawnNewCharacter _asbp_player_controller)
    (Actor|DestroyActor)))

(fn ConstructionScript)